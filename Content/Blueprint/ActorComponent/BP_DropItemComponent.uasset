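; Actor component that drops an ammo pickup beneath its owner when Drop is called.
; A short downward visibility line trace, with debug drawing left on, supplies the hit location without checking for a hit.
; It spawns PickUpActor_Ammo slightly above that point, passing its weapon type and count, adjusting for collisions or skipping the spawn if blocked.
; The component then destroys itself, so it drops only once.
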(event Custom|Drop
  (bind _returnvalue (Components|GetOwner))
  (bind _returnvalue_2 (Transformation|GetActorLocation _returnvalue))
  (bind _outhit (Collision|LineTraceByChannel _returnvalue_2 (+ _returnvalue_2 "0.000000,0.000000,-100.000000") "TraceTypeQuery1" false 0 "ForDuration" false "(R=1.000000,G=0.000000,B=0.000000,A=1.000000)" "(R=0.000000,G=1.000000,B=0.000000,A=1.000000)" 1e+01))
  (Game|SpawnActorfromClass "/Game/Blueprint/Items/PickUpActor_Ammo.PickUpActor_Ammo_C" (Math|Transform|MakeTransform (+ (.Location (Collision|BreakHitResult _outhit)) "0.000000,0.000000,20.000000")) "AdjustIfPossibleButDontSpawnIfColliding" 0 (Variables|Default|GetType) (Variables|Default|GetCout) 0)
  (Components|DestroyComponent))