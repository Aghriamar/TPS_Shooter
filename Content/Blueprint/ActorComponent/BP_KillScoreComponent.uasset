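; BP_KillScoreComponent is an actor component that awards a score when its owner dies.
; On BeginPlay it binds an event to the death notification of the owner's TPSHealthComponent.
; Its DeadOwner event reports the component's Score to BP_GameMode through EnemyDead, then destroys the component.
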(event Custom|DeadOwner
  (bind _asbp_game_mode (Utilities|Casting|CastToBP_GameMode (Game|GetGameMode)))
  ;[1 1 1] Enemy Dead
  (Default|EnemyDead _asbp_game_mode (Variables|Default|GetScore))
  (Components|DestroyComponent))

(event Custom|Destroy
  (Components|DestroyComponent))

(event EventBeginPlay
  (EventDispatchers|BindEventtoOnDead (Actor|GetComponentbyClass (Components|GetOwner) "/Script/TPS_Shooter.TPSHealthComponent") (EventDispatchers|CreateEvent :!event Custom|DeadOwner)))

(event EventTick
  (params (DeltaSeconds :type Float%20%28single-precision%29)))