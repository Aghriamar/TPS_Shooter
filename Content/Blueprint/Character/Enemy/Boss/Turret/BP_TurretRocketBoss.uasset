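; Rocket turret for the boss enemy that periodically launches missiles while its owning boss is alive.
; A looping timer checks the owner's health through its TPSHealth component, then plays the Shoot timeline or clears itself once health is depleted.
; The timeline's Shot event spawns a missile just ahead of the turret's Arrow, owned by the boss, and initializes it with hardcoded projectile and explosion settings.
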(event Custom|FireRocket
  (bind _returnvalue (Components|GetOwner))
  (bind _arrow (Variables|Default|GetArrow))
  (bind _asbp_character_enemy_boss (Utilities|Casting|CastToBP_CharacterEnemy_Boss _returnvalue))
  (bind _returnvalue_2 (Class|TPSHealthComponent|GetCurrentHealth (Variables|/Game/Blueprint/Character/Enemy/BP_EnemyBase.BP_EnemyBase_C|GetTPSHealth _asbp_character_enemy_boss)))
  (if (> _returnvalue_2 0.0)
    (Timeline|Shoot PlayFromStart
      (:Shot
        (bind _returnvalue_3 (Game|SpawnActorfromClass "/Game/Blueprint/Character/Enemy/Boss/Turret/BP_MissileTurret.BP_MissileTurret_C" (Math|Transform|MakeTransform (+ (* (Math|Vector|GetForwardVector _arrow) 1e+02) (Transformation|GetWorldLocation _arrow)) (Transformation|GetWorldRotation _arrow)) "AlwaysSpawn" _returnvalue 0))
        (Class|ProjectileDefault|InitProjectile _returnvalue_3 (Utilities|Struct|MakeProjectileInfo "/Game/Blueprint/Character/Enemy/Boss/Turret/BP_MissileTurret.BP_MissileTurret_C" "/Game/Meshes/WeaponTurrete_Boss/Missile/Hellfire_missile.Hellfire_missile" "0.000000,0.000000,0.000000|0.000000,0.000000,0.000000|1.000000,1.000000,1.000000" "/Game/Fx_Effect/Particles/P_Projectile_Trail.P_Projectile_Trail" "0.000000,0.000000,0.000000|0.000000,0.000000,0.000000|1.000000,1.000000,1.000000" 1.0 2e+01 5e+02 1e+03 "SurfaceType_Default" 0 "SurfaceType_Default" 0 0 0 3e+02 1.5e+02 3e+01 2.0))))
    (else
      (Utilities|Time|ClearandInvalidateTimerbyHandle (Variables|Default|GetFireRocket_HandlerTimer)))))

(event EventBeginPlay
  (bind _returnvalue (Utilities|Time|SetTimerbyEvent (delegate Custom|FireRocket) 3.0 true))
  (Variables|Default|SetFireRocket_HandlerTimer _returnvalue))

(fn ConstructionScript)