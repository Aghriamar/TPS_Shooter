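; Top-down player character with mouse-wheel camera zoom, walk/sprint/aim movement modes and montage-driven fire and death animations.
; The construction script configures the spring-arm camera, and the wheel changes arm length within limits, instantly or in small steps on a looping timer gated by SlideDone.
; Input flags feed ChangeMovementState; F shakes the camera and yaws the actor toward the cursor hit.
; Tick prints debug text.
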(event Custom|SlideCameraStart
  ;[1 1 1] Side Camera Start
  (Timeline|Timeline_0 PlayFromStart
    (:Finished
      (Variables|Camera|Slide|SetSlideDone true))))

(event EventTick
  (params (DeltaSeconds :type Float%20%28single-precision%29))
  ;[1 1 1] EVENT TICK
  (Development|PrintString (Utilities|String|ToString(Float) (Variables|/Script/Engine.SpringArmComponent|GetTargetArmLength (Variables|Default|GetCameraBoom))) true true "(R=0.000000,G=1.000000,B=0.106406,A=1.000000)" 0.0)
  (Development|PrintString (Utilities|String|EnumtoString (Variables|Default|GetMovementState)) true true "(R=0.000000,G=0.660000,B=1.000000,A=1.000000)" 0.0)
  (Development|PrintString "Press <Escape> to the \"Exit Game\"" true true "(R=1.000000,G=0.000000,B=0.009094,A=1.000000)" 0.0))

(event Input|ActionEvents|InputActionMovementModeChangeWalk
  (params (Key :type Key%20Structure :default "None"))
  ;[1 1 1] INPUT Movement
  (:Pressed
    (Variables|Default|SetWalkEnabled true)
    (Class|TPSShooterCharacter|ChangeMovementState :!label _label))
  (:Released
    (Variables|Default|SetWalkEnabled false)
    (goto _label)))

(event Input|ActionEvents|InputActionMovementModeChangeSprint
  (params (Key :type Key%20Structure :default "None"))
  ;[1 1 1] INPUT Movement
  (:Pressed
    (Variables|Default|SetSprintRunEnabled true)
    (Class|TPSShooterCharacter|ChangeMovementState :!label _label))
  (:Released
    (Variables|Default|SetSprintRunEnabled false)
    (goto _label)))

(event Input|AxisEvents|InputAxisMouseWheel
  (params (AxisValue :type Float%20%28single-precision%29))
  ;[1 1 1] INPUT Axis
  (if (Variables|Camera|Main|GetSlideWithSmooth)
    (CallFunction|CameraSlideSmooth AxisValue)
    (else
      (CallFunction|CameraSlide AxisValue))))

(event Input|KeyboardEvents|F
  (params (Key :type Key%20Structure :default "None"))
  ;[1 1 1] KEY F
  (:Pressed
    (CallFunction|CameraShakeEvent)
    (Transformation|SetActorRotation (Math|Rotator|MakeRotator 0.0 0.0 (.yaw (Math|Rotator|FindLookatRotation (Transformation|GetActorLocation) (.Location (Collision|BreakHitResult (.HitResult (Game|Player|GetHitResultUnderCursorbyChannel (Game|GetPlayerController 0) "TraceTypeQuery3" true))))))))))

(event Input|KeyboardEvents|SpaceBar
  (params (Key :type Key%20Structure :default "None"))
  (bind _mesh (Variables|Character|GetMesh))
  ;[1 1 1] KEY Space Bar
  (:Pressed
    (if (Variables|Default|GetAimEnabled)
      (Animation|Montage|PlayMontage _mesh "/Game/Blueprint/Character/Mannequin/Animations/NewAnim/NewFire_Rifle_Ironsights_Montage.NewFire_Rifle_Ironsights_Montage")
      (else
        (Animation|Montage|PlayMontage _mesh "/Game/Blueprint/Character/Mannequin/Animations/NewAnim/NewFire_Rifle_Hip_Montage.NewFire_Rifle_Hip_Montage")))))

(event Input|MouseEvents|RightMouseButton
  (params (Key :type Key%20Structure :default "None"))
  ;[1 1 1] INPUT Movement
  (:Pressed
    (Variables|Default|SetAimEnabled true)
    (Class|TPSShooterCharacter|ChangeMovementState :!label _label))
  (:Released
    (Variables|Default|SetAimEnabled false)
    (goto _label)))

(event Input|KeyboardEvents|V
  (params (Key :type Key%20Structure :default "None"))
  ;[1 1 1] KEY Death
  (:Pressed
    (Animation|Montage|PlayMontage (Variables|Character|GetMesh) "/Game/Blueprint/Character/Mannequin/Animations/NewAnim/NewDeath_1_Montage.NewDeath_1_Montage")))

(fn ConstructionScript
  (bind _cameraboom (Variables|Default|GetCameraBoom))
  (Variables|/Script/Engine.SpringArmComponent|SetTargetArmLength _cameraboom (Variables|Camera|Main|GetHeightCameraMin))
  (Transformation|SetRelativeRotation _cameraboom (Variables|Camera|Main|GetRotatorCamera) false false)
  (Variables|/Script/Engine.SpringArmComponent|SetbEnableCameraLag _cameraboom (Variables|Camera|Main|GetFlow))
  (Variables|/Script/Engine.SpringArmComponent|SetCameraLagSpeed _cameraboom (Variables|Camera|Main|GetCoefSmooth)))

(fn CameraShakeEvent
  (Camera|PlayWorldCameraShake "/Game/Blueprint/Game/BP_ShakeCamera.BP_ShakeCamera_C" (Transformation|GetWorldLocation (Variables|Default|GetTopDownCameraComponent)) 0.0 3e+01))

(fn CameraSlide
  (params (Value :type Float%20%28single-precision%29))
  (bind _cameraboom (Variables|Default|GetCameraBoom))
  (bind _heightcamerachangedistance (Variables|Camera|Slide|GetHeightCameraChangeDistance))
  (if (!= Value 0.0)
    (if (< Value 0.0)
      (if (>= (Variables|Camera|Main|GetHeightCameraMax) (+ (Variables|/Script/Engine.SpringArmComponent|GetTargetArmLength _cameraboom) _heightcamerachangedistance))
        (Variables|/Script/Engine.SpringArmComponent|SetTargetArmLength _cameraboom (+ (Variables|/Script/Engine.SpringArmComponent|GetTargetArmLength _cameraboom) _heightcamerachangedistance)))
      (elif (<= (Variables|Camera|Main|GetHeightCameraMin) (- (Variables|/Script/Engine.SpringArmComponent|GetTargetArmLength _cameraboom) _heightcamerachangedistance))
        (Variables|/Script/Engine.SpringArmComponent|SetTargetArmLength _cameraboom (- (Variables|/Script/Engine.SpringArmComponent|GetTargetArmLength _cameraboom) _heightcamerachangedistance))))))

(fn CameraSlideSmooth
  (params (Value :type Float%20%28single-precision%29))
  (bind _heightcamerachangedistance (Variables|Camera|Slide|GetHeightCameraChangeDistance))
  (bind _cameraboom (Variables|Default|GetCameraBoom))
  (bind _targetarmlength (Variables|/Script/Engine.SpringArmComponent|GetTargetArmLength _cameraboom))
  (if (Variables|Camera|Slide|GetSlideDone)
    (if (!= Value 0.0)
      (if (< Value 0.0)
        (if (>= (Variables|Camera|Main|GetHeightCameraMax) (+ _targetarmlength _heightcamerachangedistance))
          (Variables|Camera|Slide|SetSlideUp true)
          (Variables|Camera|Slide|SetSlideDone false :!label _label)
          (bind _returnvalue (Utilities|Time|SetTimerbyFunctionName 0 "CameraSlideSmoothTick" (Variables|Camera|Slide|GetTimerStep) true))
          (Variables|Camera|Slide|SetSlideTimer _returnvalue))
        (elif (<= (Variables|Camera|Main|GetHeightCameraMin) (- _targetarmlength _heightcamerachangedistance))
          (Variables|Camera|Slide|SetSlideUp false)
          (goto _label))))))

(fn CameraSlideSmoothTick
  (bind _heightcamerachangeslidestepdistance (Variables|Camera|Slide|GetHeightCameraChangeSlideStepDistance))
  (bind _cameraboom (Variables|Default|GetCameraBoom))
  (bind _output_get (Variables|Camera|Slide|SetCurrentSlideDistance (+ (Variables|Camera|Slide|GetCurrentSlideDistance) _heightcamerachangeslidestepdistance)))
  (Variables|/Script/Engine.SpringArmComponent|SetTargetArmLength _cameraboom (select (Variables|Camera|Slide|GetSlideUp) (+ (Variables|/Script/Engine.SpringArmComponent|GetTargetArmLength _cameraboom) _heightcamerachangeslidestepdistance) (- (Variables|/Script/Engine.SpringArmComponent|GetTargetArmLength _cameraboom) _heightcamerachangeslidestepdistance)))
  (if (>= _output_get (Variables|Camera|Slide|GetHeightCameraChangeDistance))
    (Variables|Camera|Slide|SetCurrentSlideDistance 0.0)
    (Variables|Camera|Slide|SetSlideDone true)
    (Utilities|Time|ClearandInvalidateTimerbyHandle (Variables|Camera|Slide|GetSlideTimer))))