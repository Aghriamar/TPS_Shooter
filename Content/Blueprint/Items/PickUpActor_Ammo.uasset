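; Ammo pickup actor that grants a set amount of ammo for one weapon type to an overlapping character's inventory.
; On BeginPlay, InitActor selects a magazine or grenade mesh and a colored ring particle by ammo type, destroying either component when no asset is assigned.
; The character overlap event checks whether the inventory can take that ammo, then changes the ammo slot and triggers pickup success.
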(event EventBeginPlay
  (|CallParentFunction)
  (CallFunction|InitActor))

(event Collision|EventActorBeginOverlap
  (params (OtherActor :type Actor%20Object%20Reference))
  (|CallParentFunction OtherActor) ; This node is disabled and will not be called.\nDrag off pins to build functionality.
)

(event EventTick
  (params (DeltaSeconds :type Float%20%28single-precision%29))
  (|CallParentFunction DeltaSeconds) ; This node is disabled and will not be called.\nDrag off pins to build functionality.
)

(event EventOverlapCharacter
  (params (ToInventory :type TPS%20Inventory%20Component%20Object%20Reference))
  (bind _weapontypeammo (Variables|Default|GetWeaponTypeAmmo))
  (bind _returnvalue (Class|TPSInventoryComponent|CheckCanTakeAmmo ToInventory _weapontypeammo))
  (if _returnvalue
    (Class|TPSInventoryComponent|AmmoSlotChangeValue ToInventory _weapontypeammo (Variables|Default|GetCout))
    (CallFunction|PickUpSuccess)))

(fn ConstructionScript
  (|CallParentFunction))

(fn InitActor
  (params (InfoActor :type Drop%20Item%20Structure))
  (bind _weapontypeammo (Variables|Default|GetWeaponTypeAmmo))
  (bind _staticmesh (Variables|Default|GetStaticMesh))
  (bind _particlesystem (Variables|Default|GetParticleSystem))
  (bind _returnvalue (Utilities|Select :Index _weapontypeammo :RifleType "/Game/Fx_Effect/Particles/Items/P_Ring_Yellow.P_Ring_Yellow" :ShotGunType "/Game/Fx_Effect/Particles/Items/P_Ring_red.P_Ring_Red" :SniperRifle "/Game/Fx_Effect/Particles/Items/P_Ring_Purple.P_Ring_Purple" :GrenadeLauncher "/Game/Fx_Effect/Particles/Items/P_Ring_Green.P_Ring_Green" :RocketLauncher "/Game/Fx_Effect/Particles/Items/P_Ring_Blue.P_Ring_Blue"))
  (bind _returnvalue_2 (Utilities|Select :Index _weapontypeammo :RifleType "/Game/FPS_Weapon_Bundle/Weapons/Meshes/AR4/SM_AR4_Mag_Empty.SM_AR4_Mag_Empty" :ShotGunType "/Game/FPS_Weapon_Bundle/Weapons/Meshes/SMG11/SM_SMG11_Mag_Empty_X.SM_SMG11_Mag_Empty_X" :SniperRifle "/Game/FPS_Weapon_Bundle/Weapons/Meshes/KA74U/SM_KA74U_Mag_Empty_X.SM_KA74U_Mag_Empty_X" :GrenadeLauncher "/Game/FPS_Weapon_Bundle/Weapons/Meshes/G67_Grenade/SM_G67.SM_G67" :RocketLauncher 0))
  (Utilities|FlowControl|Sequence
    (:then_0
      (Utilities|IsValid _returnvalue_2
        (:Is%20Valid
          (Components|StaticMesh|SetStaticMesh _staticmesh _returnvalue_2)
          (Transformation|SetRelativeLocation _staticmesh "0, 0, 0" false false)
          (Transformation|SetRelativeScale3D _staticmesh "2.000000,2.000000,2.000000")
          (Transformation|SetRelativeRotation _staticmesh (Math|Rotator|MakeRotator -9e+01 0.0 9e+01) false false))
        (:Is%20Not%20Valid
          (Components|DestroyComponent _staticmesh))))
    (:then_1
      (Utilities|IsValid _returnvalue
        (:Is%20Valid
          (Effects|Components|ParticleSystem|SetTemplate _particlesystem _returnvalue)
          (Transformation|SetRelativeScale3D _particlesystem "1.000000,1.000000,1.000000"))
        (:Is%20Not%20Valid
          (Components|DestroyComponent _particlesystem))))))