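; Weapon pickup actor that gives its weapon to an overlapping character's inventory.
; On BeginPlay it looks up drop info by ItemName in BP_GameInstance, then InitActor sets a static or fallback skeletal mesh and particle, destroying components left without assets.
; On overlap it tries adding the weapon to inventory; failure starts a weapon-switch on the character, which ends when the sphere overlap ends.
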(event OnComponentEndOverlap(Sphere)
  (params (OverlappedComponent :type Primitive%20Component%20Object%20Reference) (OtherActor :type Actor%20Object%20Reference) (OtherComp :type Primitive%20Component%20Object%20Reference) (OtherBodyIndex :type Integer))
  (bind _asbp_character (Utilities|Casting|CastToBP_Character OtherActor))
  (Default|EndSwitchWeapon _asbp_character))

(event EventBeginPlay
  (bind _itemname (Variables|Default|GetItemName))
  (|CallParentFunction)
  (if (Utilities|Name|NotEqual(Name) _itemname "None")
    (bind _asbp_game_instance (Utilities|Casting|CastToBP_GameInstance (Game|GetGameInstance)))
    (bind (_outinfo _returnvalue) (Class|TPSShooterGameInstance|GetDropItemInfobyName _asbp_game_instance _itemname))
    (if _returnvalue
      (Variables|Default|SetWeaponInfo _outinfo)))
  (CallFunction|InitActor (Variables|Default|GetWeaponInfo)))

(event Collision|EventActorBeginOverlap
  (params (OtherActor :type Actor%20Object%20Reference))
  (|CallParentFunction OtherActor) ; This node is disabled and will not be called.\nDrag off pins to build functionality.
)

(event EventTick
  (params (DeltaSeconds :type Float%20%28single-precision%29))
  (|CallParentFunction DeltaSeconds) ; This node is disabled and will not be called.\nDrag off pins to build functionality.
)

(event EventOverlapCharacter
  (params (ToInventory :type TPS%20Inventory%20Component%20Object%20Reference))
  (|CallParentFunction ToInventory)
  (bind _returnvalue (Class|TPSInventoryComponent|TryGetWeapontoInventory ToInventory (Utilities|Struct|BreakDropItem (Variables|Default|GetWeaponInfo))))
  (if _returnvalue
    (CallFunction|PickUpSuccess)
    (else
      (bind _asbp_character (Utilities|Casting|CastToBP_Character (Components|GetOwner ToInventory)))
      (Default|StartSwitchWeapon _asbp_character self))))

(fn ConstructionScript
  (|CallParentFunction))

(fn InitActor
  (params (InfoActor :type Drop%20Item%20Structure))
  (bind (_weaponstaticmesh _weaponskeletmesh _particleitem _offset _weaponinfo) (Utilities|Struct|BreakDropItem InfoActor))
  (bind _particlesystem (Variables|Default|GetParticleSystem))
  (bind _weaponstaticmesh_2 (Variables|Default|GetWeaponStaticMesh))
  (bind _weaponskeletalmesh (Variables|Default|GetWeaponSkeletalMesh))
  (Utilities|FlowControl|Sequence
    (:then_0
      (Utilities|IsValid _weaponstaticmesh
        (:Is%20Valid
          (Components|StaticMesh|SetStaticMesh _weaponstaticmesh_2 _weaponstaticmesh)
          (Transformation|SetRelativeLocation _weaponstaticmesh_2 (.location _offset) false false)
          (Transformation|SetRelativeRotation _weaponstaticmesh_2 (.rotation _offset) false false))
        (:Is%20Not%20Valid
          (Components|DestroyComponent _weaponstaticmesh_2)
          (Utilities|IsValid _weaponskeletmesh
            (:Is%20Valid
              (Class|SkinnedMeshComponent|SetSkeletalMesh _weaponskeletalmesh _weaponskeletmesh true)
              (Transformation|SetRelativeLocation _weaponskeletalmesh (.location _offset) false false)
              (Transformation|SetRelativeRotation _weaponskeletalmesh (.rotation _offset) false false))
            (:Is%20Not%20Valid
              (Components|DestroyComponent _weaponskeletalmesh)
              (Development|PrintString "Error Drop Item Not have any MESH"))))))
    (:then_1
      (Utilities|IsValid _particleitem
        (:Is%20Valid
          (Effects|Components|ParticleSystem|SetTemplate _particlesystem _particleitem)
          (Transformation|SetRelativeScale3D _particlesystem (.scale _offset)))
        (:Is%20Not%20Valid
          (Components|DestroyComponent _particlesystem))))))