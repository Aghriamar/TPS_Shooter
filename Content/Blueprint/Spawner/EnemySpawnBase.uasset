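; Base enemy spawn point that registers itself with BP_GameMode on BeginPlay.
; Boss points set themselves as the game mode's single boss spawn point.
; Other points take the first digit found in the string form of their Phase value and use it as an index to add themselves to one of five per-phase spawn point lists.
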(event EventBeginPlay
  (CallFunction|RegistPoint))

(fn ConstructionScript)

(fn RegistPoint
  (if (Variables|Default|GetbIsBoss)
    (bind _asbp_game_mode (Utilities|Casting|CastToBP_GameMode (Game|GetGameMode)))
    (Variables|/Game/Blueprint/Game/BP_GameMode.BP_GameMode_C|SetSpawnPointBoss _asbp_game_mode self)
    (else
      (bind _array_element (Utilities|Array|ForEachLoopwithBreak (Utilities|String|GetCharacterArrayfromString (Utilities|String|ToString(Name) (Variables|Default|GetPhase))) :!label _label)
        (:LoopBody
          (if (Class|KismetStringLibrary|IsNumeric _array_element)
            (LocalVariables|SetCurrentPhasePoint (Math|Conversions|ToInteger(Byte) _array_element))
            (goto _label Break)))
        (:Completed
          (bind _asbp_game_mode_2 (Utilities|Casting|CastToBP_GameMode (Game|GetGameMode)))
          (Utilities|Array|Add (Utilities|Select :Index (LocalVariables|GetCurrentPhasePoint) :Option%200 (Variables|/Game/Blueprint/Game/BP_GameMode.BP_GameMode_C|GetSpawnPointPhase1 _asbp_game_mode_2) :Option%201 (Variables|/Game/Blueprint/Game/BP_GameMode.BP_GameMode_C|GetSpawnPointPhase2 _asbp_game_mode_2) :Option%202 (Variables|/Game/Blueprint/Game/BP_GameMode.BP_GameMode_C|GetSpawnPointPhase3 _asbp_game_mode_2) :Option%203 (Variables|/Game/Blueprint/Game/BP_GameMode.BP_GameMode_C|GetSpawnPointPhase4 _asbp_game_mode_2) :Option%204 (Variables|/Game/Blueprint/Game/BP_GameMode.BP_GameMode_C|GetSpawnPointPhase5 _asbp_game_mode_2)) self))))))