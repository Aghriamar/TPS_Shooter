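; BP_GameState tracks remaining lives, score and the current phase of the game.
; CanPlayerRespawn consumes a life on each call and reports whether any remained, along with the current phase.
; IncrementScore updates the score and pushes it to the first player controller's stats widget.
; It advances the phase when the score reaches that phase's PhaseWinScore threshold, returning true once the last phase is passed.
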(event EventBeginPlay)

(event EventTick
  (params (DeltaSeconds :type Float%20%28single-precision%29)))

(fn ConstructionScript)

(fn CanPlayerRespawn
  (bind _coutlives (Variables|Default|GetCoutLives))
  (Math|Integer|DecrementInt _coutlives
    (:%20%20
      (return (>= _coutlives 0) (Variables|Default|GetCurrentPhase)))))

(fn IncrementScore
  (params (ChangeValue :type Integer))
  (bind _phasewinscore (Variables|Default|GetPhaseWinScore))
  (bind _output_get (Variables|Default|SetScore (+ (Variables|Default|GetScore) ChangeValue)))
  (bind _asbp_player_controller (Utilities|Casting|CastToBP_PlayerController (Game|GetPlayerController 0)))
  (Default|SetScoreText (Variables|/Game/Blueprint/Widget/IngameWidget.IngameWidget_C|GetBPW_Stats (Variables|/Game/Blueprint/Game/BP_PlayerController.BP_PlayerController_C|GetIngameWidget _asbp_player_controller)) _output_get)
  (if (Utilities|Array|IsValidIndex _phasewinscore (Variables|Default|GetCurrentPhase))
    (if (<= (Utilities|Array|Get(acopy) _phasewinscore (Variables|Default|GetCurrentPhase)) (Variables|Default|GetScore))
      (Variables|Default|SetCurrentPhase (+ (Variables|Default|GetCurrentPhase) 1))
      (if (not (Utilities|Array|IsValidIndex _phasewinscore (Variables|Default|GetCurrentPhase)))
        (return true)))
    (else
      (Development|PrintString "Wrong Current Phase not valid"))))