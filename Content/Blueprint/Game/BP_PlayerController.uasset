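; Player controller Blueprint that drives the possessed pawn's movement and quits the game on Escape.
; Forward and right axis inputs add movement along the pawn's own forward and right vectors.
; Rightward movement requires a BP_Character pawn and is blocked while its SprintRunEnabled flag is on, so sprinting allows no strafing.
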(event EventBeginPlay)

(event EventTick
  (params (DeltaSeconds :type Float%20%28single-precision%29)))

(event Input|AxisEvents|InputAxisMoveForward
  (params (AxisValue :type Float%20%28single-precision%29))
  (bind _returnvalue (Game|Player|GetPlayerPawn 0))
  (Pawn|Input|AddMovementInput _returnvalue (Transformation|GetActorForwardVector _returnvalue) AxisValue false))

(event Input|AxisEvents|InputAxisMoveRight
  (params (AxisValue :type Float%20%28single-precision%29))
  (bind _returnvalue (Game|Player|GetPlayerPawn 0))
  (bind _asbp_character (Utilities|Casting|CastToBP_Character _returnvalue))
  (if (not (Variables|/Script/TPS_Shooter.TPS_ShooterCharacter|GetSprintRunEnabled _asbp_character))
    (Pawn|Input|AddMovementInput _returnvalue (Transformation|GetActorRightVector _returnvalue) AxisValue false)))

(event Input|KeyboardEvents|Escape
  (params (Key :type Key%20Structure :default "None"))
  (:Pressed
    (Game|QuitGame 0 "Quit" false)))

(fn ConstructionScript)