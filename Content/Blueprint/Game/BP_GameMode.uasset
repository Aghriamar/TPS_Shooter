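; Game mode that runs phase-based enemy spawning, player respawns and the win screen, relying on BP_GameState for score, enemy count and current phase.
; A looping timer draws enemy classes from a shuffled pool, refilled from the master list, and spawns them at random per-phase points or boxes.
; Scoring kills can trigger the end-game widget.
; Phase changes kill living enemies without score and refill the pool.
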(event EventBeginPlay
  (Utilities|Time|SetTimerbyFunctionName 0 "TryRespawnEnemy" 1.0 true))

(event EventTick
  (params (DeltaSeconds :type Float%20%28single-precision%29)))

(fn ConstructionScript)

(fn TrytoRespawnPlayer
  (bind _returnvalue (Game|GetPlayerController 0))
  (bind _asbp_game_state (Utilities|Casting|CastToBP_GameState (Game|GetGameState)))
  (bind (_success _currentphase) (Default|CanPlayerRespawn _asbp_game_state))
  (if _success
    (Class|GameModeBase|RestartPlayeratPlayerStart _returnvalue (Class|GameModeBase|FindPlayerStart _returnvalue (Utilities|Select :Index _currentphase :Option%200 "Phase0" :Option%201 "Phase1" :Option%202 "Phase2" :Option%203 "Phase3" :Option%204 "Phase4")))
    (return true)
    (else
      (return _success))))

(fn ChoosePlayerStart
  (params (Player :type Controller%20Object%20Reference))
  (return (Class|GameModeBase|FindPlayerStart Player "Phase0")))

(fn EnemyDead
  (params (Score :type Integer))
  (if (> Score 0)
    (bind _asbp_game_state (Utilities|Casting|CastToBP_GameState (Game|GetGameState)))
    (bind _biswin (Default|IncrementScore _asbp_game_state Score))
    (Default|IncrementEnemy _asbp_game_state -1)
    (if _biswin
      (bind _returnvalue (UserInterface|CreateWidget "/Game/Blueprint/Widget/BPW_EndGame.BPW_EndGame_C" 0 true))
      (UserInterface|Viewport|AddtoViewport _returnvalue 0)
      (Variables|/Script/Engine.PlayerController|SetbShowMouseCursor (Game|GetPlayerController 0) true))))

(fn CheckWinCondition)

(fn TryRespawnEnemy
  (bind _currentspawnpool (Variables|Default|GetCurrentSpawnPool))
  (bind _asbp_game_state (Utilities|Casting|CastToBP_GameState (Game|GetGameState)))
  (bind _valid (Default|CheckEnemyforPhase _asbp_game_state))
  (if _valid
    (if (> (Utilities|Array|Length (Variables|Default|GetCurrentSpawnPool)) 0) :!label _label
      (LocalVariables|SetClassToSpawn (Utilities|Array|Get(acopy) _currentspawnpool))
      (Utilities|Array|RemoveIndex _currentspawnpool)
      (bind _output_get (LocalVariables|SetCurrentPoint (Utilities|Array|Get(acopy) (Utilities|Select :Index (Variables|/Game/Blueprint/Game/BP_GameState.BP_GameState_C|GetCurrentPhase _asbp_game_state) :Option%200 (Variables|Default|GetSpawnPointPhase1) :Option%201 (Variables|Default|GetSpawnPointPhase2) :Option%202 (Variables|Default|GetSpawnPointPhase3) :Option%203 (Variables|Default|GetSpawnPointPhase4) :Option%204 (Variables|Default|GetSpawnPointPhase5)) (Math|Random|RandomIntegerinRange 0 (- (Utilities|Array|Length (Utilities|Select :Index (Variables|/Game/Blueprint/Game/BP_GameState.BP_GameState_C|GetCurrentPhase _asbp_game_state) :Option%200 (Variables|Default|GetSpawnPointPhase1) :Option%201 (Variables|Default|GetSpawnPointPhase2) :Option%202 (Variables|Default|GetSpawnPointPhase3) :Option%203 (Variables|Default|GetSpawnPointPhase4) :Option%204 (Variables|Default|GetSpawnPointPhase5))) 1)))))
      (if (Variables|/Game/Blueprint/Spawner/EnemySpawnBase.EnemySpawnBase_C|GetbIsPoint _output_get)
        (Game|SpawnActorfromClass (LocalVariables|GetClassToSpawn) (Math|Conversions|ToTransform(Vector) (Transformation|GetActorLocation _output_get)) "AdjustIfPossibleButDontSpawnIfColliding" 0 0)
        (else
          (Game|SpawnActorfromClass (LocalVariables|GetClassToSpawn) (Math|Conversions|ToTransform(Vector) (Math|Random|RandomPointinBoundingBox (Transformation|GetActorLocation _output_get) (Variables|/Script/Engine.BoxComponent|GetBoxExtent (Variables|/Game/Blueprint/Spawner/EnemySpawnBase.EnemySpawnBase_C|GetBox _output_get)))) "AlwaysSpawn" 0 0)))
      (Default|IncrementEnemy _asbp_game_state 1)
      (else
        (Development|PrintString "Spawn Pool is Empty! Refilling...")
        (CallFunction|RefillSpawnPool)
        (goto _label)))))

(fn NextPhaseStart
  (params (CurrentPhase :type Integer))
  (bind _outactors (Actor|GetAllActorsOfClass "/Game/Blueprint/Character/Enemy/BP_EnemyBase.BP_EnemyBase_C"))
  (for _array_element _outactors
    (if (not (Variables|/Game/Blueprint/Character/Enemy/BP_EnemyBase.BP_EnemyBase_C|GetbIsDead _array_element))
      (Default|Destroy (Variables|/Game/Blueprint/Character/Enemy/BP_EnemyBase.BP_EnemyBase_C|GetBP_KillScoreComponent _array_element))
      (Game|Damage|ApplyDamage _array_element 5e+03 0 0)))
  (CallFunction|RefillSpawnPool))

(fn RefillSpawnPool
  (bind _currentspawnpool (Variables|Default|GetCurrentSpawnPool))
  (Utilities|Array|Clear _currentspawnpool)
  (for _array_element (Variables|Default|GetMasterEnemyList)
    (Utilities|Array|Add _currentspawnpool _array_element))
  (Utilities|Array|Shuffle _currentspawnpool))