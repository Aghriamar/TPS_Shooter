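; BP_LobbyState is the lobby state object that tracks which colors are blocked for selection.
; Server-side color swaps and single add/remove events update BlockColor, then send it to every BP_LobbyPlayerController listed in BP_LobbyMode to refresh lobby widgets.
; Getters return the blocked colors and the available ones, found by filtering AllColor against BlockColor.
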(event Custom|SelectedNewColor_OnServer
  (params (Remove :type Material%20Interface%20Object%20Reference) (Add :type Material%20Interface%20Object%20Reference))
  (bind _blockcolor (Variables|Default|GetBlockColor))
  (Utilities|Array|RemoveItem _blockcolor Remove)
  (Utilities|Array|Add _blockcolor Add)
  (bind _asbp_lobby_mode (Utilities|Casting|CastToBP_LobbyMode (Game|GetGameMode)))
  (for _array_element (Variables|/Game/Blueprint/Game/Lobby/BP_LobbyMode.BP_LobbyMode_C|GetPlayerController _asbp_lobby_mode)
    (bind _asbp_lobby_player_controller (Utilities|Casting|CastToBP_LobbyPlayerController _array_element))
    (Default|UpdateColorsLobbyWidgetonClient _asbp_lobby_player_controller (Variables|Default|GetBlockColor))))

(event Custom|AddOrRemoveColorToBlock
  (params (Color :type Material%20Interface%20Object%20Reference) (IsRemove :type Boolean))
  (bind _blockcolor (Variables|Default|GetBlockColor))
  (if IsRemove
    (Utilities|Array|RemoveItem _blockcolor Color)
    (else
      (Utilities|Array|Add _blockcolor Color)))
  (bind _asbp_lobby_mode (Utilities|Casting|CastToBP_LobbyMode (Game|GetGameMode)))
  (for _array_element (Variables|/Game/Blueprint/Game/Lobby/BP_LobbyMode.BP_LobbyMode_C|GetPlayerController _asbp_lobby_mode)
    (bind _asbp_lobby_player_controller (Utilities|Casting|CastToBP_LobbyPlayerController _array_element))
    (Default|UpdateColorsLobbyWidgetonClient _asbp_lobby_player_controller (Variables|Default|GetBlockColor))))

(fn ConstructionScript)

(fn GetAviableColor
  (for _array_element (Variables|Default|GetAllColor)
    (LocalVariables|SetCanTake true)
    (bind _array_element_2 (Utilities|Array|ForEachLoopwithBreak (Variables|Default|GetBlockColor) :!label _label)
      (:LoopBody
        (if (== _array_element_2 _array_element)
          (LocalVariables|SetCanTake false)
          (goto _label Break)))
      (:Completed
        (if (LocalVariables|GetCanTake)
          (Utilities|Array|Add (LocalVariables|GetAviableColor) _array_element)))))
  (return (LocalVariables|GetAviableColor)))

(fn GetBlockColor
  (return (Variables|Default|GetBlockColor)))