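; Lobby player controller that runs the menu and links each player to the game mode and their lobby character.
; On local start it switches view to a camera actor and opens BPW_LobbyMenu; the host builds level buttons from DT_Levels and defaults to the first.
; Map and color picks pass to BP_LobbyMode, while other events update the widget or drive the saved character's FX, readiness and color.
; On authority, destruction also removes that character.
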(event Custom|UpdateMeReady
  (Default|MeReadyMulticast (Variables|Default|GetLobbyCharacter)))

(event Custom|UpdatePlayerSelectedMap
  (params (CurrentLevelByServer :type Name))
  (bind _asbp_lobby_mode (Utilities|Casting|CastToBP_LobbyMode (Game|GetGameMode)))
  (Default|UpdateLevelName _asbp_lobby_mode CurrentLevelByServer))

(event Custom|UpdateLobbyWidgetOnClient
  (params (Name :type Name))
  (Default|UpdateLevelName (Variables|Default|GetLobbyMenu) Name))

(event Custom|UpdatePlayerName
  (params (InText :type Text))
  (bind _lobbymenu (Variables|Default|GetLobbyMenu))
  (Utilities|IsValid _lobbymenu
    (:Is%20Valid
      (Rendering|Components|TextRender|SetText (Variables|/Game/Blueprint/Widget/Menu/LobbyMenu/BPW_LobbyMenu.BPW_LobbyMenu_C|GetTextBlock_NamePlayer _lobbymenu) (Utilities|Text|ToText(String) (Utilities|String|GetSubstring (Utilities|String|ToString(Text) InText) 0 11))))))

(event Custom|SelectedNewColor
  (params (Color :type Material%20Interface%20Object%20Reference))
  (bind _asbp_lobby_mode (Utilities|Casting|CastToBP_LobbyMode (Game|GetGameMode)))
  (Default|UpdateColorforCharacter _asbp_lobby_mode Color self))

(event Custom|SaveLobbyCgaracter
  (params (LobbyCharacter :type BP%20Lobby%20Characer%20Object%20Reference))
  (Variables|Default|SetLobbyCharacter LobbyCharacter))

(event Custom|UpdateColorsLobbyWidget_OnClient
  (params (BlocksColors :type Array%20of%20Material%20Interface%20Object%20References))
  (bind _lobbymenu (Variables|Default|GetLobbyMenu))
  (Utilities|IsValid _lobbymenu
    (:Is%20Valid
      (Default|UpdateAviableColor _lobbymenu BlocksColors))))

(event Custom|UpdateLobbyCharacterColorParam
  (params (NewColor :type Material%20Interface%20Object%20Reference))
  (Default|ChangeColoronServer (Variables|Default|GetLobbyCharacter) NewColor))

(event Custom|RemoveAllWidget
  (Viewport|RemoveAllWidgets))

(event Custom|UpdateSpawnFX
  (Default|SpawnFX (Variables|Default|GetLobbyCharacter)))

(event EventBeginPlay
  (bind _returnvalue (Networking|IsServer))
  (Utilities|FlowControl|Delay 0.2)
  (if (Pawn|IsLocalPlayerController)
    (Variables|Default|SetbShowMouseCursor true)
    (bind _returnvalue_2 (Actor|GetActorOfClass "/Script/Engine.CameraActor"))
    (Game|Player|SetViewTargetwithBlend _returnvalue_2 0.0 "VTBlend_Linear" 0.0 false)
    (bind _returnvalue_3 (UserInterface|CreateWidget "/Game/Blueprint/Widget/Menu/LobbyMenu/BPW_LobbyMenu.BPW_LobbyMenu_C" 0 _returnvalue "" "None"))
    (Variables|Default|SetLobbyMenu _returnvalue_3)
    (UserInterface|Viewport|AddtoViewport _returnvalue_3 0)
    (if _returnvalue
      (bind _outrownames (DataTable|GetDataTableRowNames "/Game/Blueprint/Table/DT_Levels.DT_Levels"))
      (bind _returnvalue_4 (Utilities|GetDataTableRow "/Game/Blueprint/Table/DT_Levels.DT_Levels" (Utilities|Array|Get(acopy) _outrownames))
        (:then
          (Default|UpdateLevelName (Variables|Default|GetLobbyMenu) (.LevelName (Utilities|Struct|BreakF_Level _returnvalue_4)))
          (CallFunction|UpdatePlayerSelectedMap (.LevelName (Utilities|Struct|BreakF_Level _returnvalue_4)))
          (for _array_element _outrownames
            (bind _returnvalue_5 (Utilities|GetDataTableRow "/Game/Blueprint/Table/DT_Levels.DT_Levels" _array_element)
              (:then
                (bind _returnvalue_6 (UserInterface|CreateWidget "/Game/Blueprint/Widget/Menu/LobbyMenu/BPW_LobbyLevelButton.BPW_LobbyLevelButton_C" 0 (.LevelName (Utilities|Struct|BreakF_Level _returnvalue_5)) (Variables|Default|GetLobbyMenu)))
                (Class|VerticalBox|AddChildtoVerticalBox (Variables|/Game/Blueprint/Widget/Menu/LobbyMenu/BPW_LobbyMenu.BPW_LobbyMenu_C|GetSelectLevelByHostBox (Variables|Default|GetLobbyMenu)) _returnvalue_6))
              (:RowNotFound
                (Development|PrintString "Check Table level" true true "(R=1.000000,G=0.000000,B=0.000000,A=1.000000)")))))
        (:RowNotFound
          (Development|PrintString "Check Table level" true true "(R=1.000000,G=0.000000,B=0.000000,A=1.000000)")))
      (else
        (Default|UpdateLevelName _returnvalue_3 (Variables|Default|GetCurrentLevelByServer))))))

(event EventDestroyed
  (Networking|SwitchHasAuthority
    (:Authority
      (Actor|DestroyActor (Variables|Default|GetLobbyCharacter)))))

(fn ConstructionScript)