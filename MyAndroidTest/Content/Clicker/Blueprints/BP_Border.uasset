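; BP_Border is a rotating border actor in the Clicker game that updates the life display when hit.
; On BeginPlay it caches the player's BP_Hud.
; UpdateRotationRate adds the supplied value to the RotatingMovement component's current yaw rate, so successive calls accumulate.
; OnHit calls UpdateLife on the HUD's UI, leaving life handling to that widget.
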(event Custom|UpdateRotationRate
  (params (RotationRate :type Float%20%28single-precision%29))
  (Variables|/Script/Engine.RotatingMovementComponent|SetRotationRate (Variables|Default|GetRotatingMovement) (Math|Rotator|MakeRotator 0.0 0.0 (+ RotationRate (.yaw (Variables|/Script/Engine.RotatingMovementComponent|GetRotationRate (Variables|Default|GetRotatingMovement)))))))

(event EventBeginPlay
  (bind _asbp_hud (Utilities|Casting|CastToBP_Hud (HUD|GetHUD (Game|GetPlayerController 0))))
  (Variables|Default|SetBP_Hud _asbp_hud))

(event Collision|EventActorBeginOverlap
  (params (OtherActor :type Actor%20Object%20Reference)))

(event EventTick
  (params (DeltaSeconds :type Float%20%28single-precision%29)))

(event EventOnHit
  (params (HitComponent :type Primitive%20Component%20Object%20Reference))
  (Default|UpdateLife (Variables|/Game/Clicker/Blueprints/BP_Hud.BP_Hud_C|GetUI (Variables|Default|GetBP_Hud))))

(fn ConstructionScript)