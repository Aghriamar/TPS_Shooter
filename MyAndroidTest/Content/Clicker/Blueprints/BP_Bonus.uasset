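; BP_Bonus is a hittable pickup for the clicker game that acts as a true or false bonus, based on IsTrueBonus.
; The construction script uses that flag to pick a cube or cone mesh and tints it green or red through a dynamic material instance.
; OnHit passes a negative value for true bonuses, or a positive one for false, to BPBorder's UpdateRotationRate, then destroys the actor.
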(event EventBeginPlay)

(event Collision|EventActorBeginOverlap
  (params (OtherActor :type Actor%20Object%20Reference)))

(event EventTick
  (params (DeltaSeconds :type Float%20%28single-precision%29)))

(event EventOnHit
  (params (HitComponent :type Primitive%20Component%20Object%20Reference))
  (Default|UpdateRotationRate (Variables|Default|GetBP_Border) (Math|Float|SelectFloat -1e+01 1e+01 (Variables|Default|GetbIsTrueBonus)))
  (Actor|DestroyActor))

(fn ConstructionScript
  (Components|StaticMesh|SetStaticMesh (Variables|Default|GetStaticMesh) (select (Variables|Default|GetbIsTrueBonus) "/Game/Geometry/Meshes/1M_Cube.1M_Cube" "/Engine/BasicShapes/Cone.Cone"))
  (Rendering|Material|SetMaterial (Variables|Default|GetStaticMesh) 0 "/Game/Clicker/Materials/MM_Color.MM_Color")
  (bind _returnvalue (Rendering|Material|CreateDynamicMaterialInstance (Variables|Default|GetStaticMesh) 0 "/Game/Clicker/Materials/MM_Color.MM_Color" "None" :!class /Script/Engine.PrimitiveComponent))
  (Rendering|Material|SetVectorParameterValue _returnvalue "Color" (Math|Color|SelectColor "(R=0.000000,G=1.000000,B=0.025071,A=1.000000)" "(R=1.000000,G=0.028078,B=0.000000,A=1.000000)" (Variables|Default|GetbIsTrueBonus)) :!class /Script/Engine.MaterialInstanceDynamic))